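; Crab pot placeable that catches items over time and through bait-based crafting.
; A looping timer runs passive catches from the insect weight table, while FishCaught picks a table by the bait among a recipe's ingredients.
; Both roll 1-100 against map values as cumulative thresholds, then add the result if a free slot or unfilled stack exists.
; On inventory changes, the server deletes one item of a hardcoded template.
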(event `self.ReceiveBeginPlay`
  (`|ExecutionSequence`
    (:`then_0`
      (bind _returnvalue (`KismetSystemLibrary.K2_SetTimerDelegate` (delegate `Tick`) (* (`self.Tick Time`) (`self.Tick modifier`)) true))
      (set `self.TimerHandle` _returnvalue))
    (:`then_1`
      (add `CraftingQueue.SignalRecipeCrafted` (`self.CraftingQueue`) (`|CreateDelegate` :!event `FishCaught`)))))

(event `Tick`
  (if (not (`self.IsABrush`))
    (`self.PassiveCatch`)))

(event `self.PlaceableInventory.SignalItemAdded`
  (params (index :type Integer) (item :type "GameItem Object Reference") (srcInventory :type "ItemInventory Object Reference") (srcIndex :type Integer))
  (if (`KismetSystemLibrary.IsServer`)
    (`ItemInventory.DeleteItemsByTemplate` (`self.PlaceableInventory`) 13599 1 :!label _label)))

(event `self.PlaceableInventory.SignalItemRemoved`
  (params (index :type Integer) (item :type "GameItem Object Reference") (dstInventory :type "ItemInventory Object Reference") (dstIndex :type Integer))
  (if (`KismetSystemLibrary.IsServer`)
    (goto _label)))

(fn `FishCaught`
  (params (NewParam :type "RecipeItem Object Reference"))
  (locals (BaitItemID :type "Array of Integer") (BaitIndex :type Integer) (SpawnWeights :type "Map of Integer to Integer") (ChanceResult :type Integer) (ItemToSpawn :type Integer))
  (for _array_element (`RecipeItem.Ingredients` NewParam)
    (bind _returnvalue (`KismetArrayLibrary.Array_Find` (`local.BaitItemID`) (`.IngredientID` (break `IngredientEntry` _array_element))))
    (if (>= _returnvalue 0)
      (set `local.BaitIndex` _returnvalue)
      (break)))
  (set `local.SpawnWeights` (select `int` (`local.BaitIndex`) :`0` (`self.InsectSpawnWeights`) :`1` (`self.GrubSpawnWeights`) :`2` (`self.WorkerBeeSpawnWeights`) :`3` (`self.QueenBeeSpawnWeights`)))
  (set `local.ChanceResult` (`KismetMathLibrary.RandomIntegerInRange` 1 100))
  (bind _values (`BlueprintMapLibrary.Map_Values` (`local.SpawnWeights`)))
  (for (_array_element_2 _array_index) _values
    (if (<= (`local.ChanceResult`) _array_element_2)
      (bind _keys (`BlueprintMapLibrary.Map_Keys` (`local.SpawnWeights`)))
      (set `local.ItemToSpawn` (`KismetArrayLibrary.Array_Get` _keys _array_index))
      (break)))
  (`self.SpawnResultItem` (`local.ItemToSpawn`)))

(fn `GetArtisanThrallInventory`
  (returns (ReturnValue :type "ItemInventory Object Reference"))
  (return null))

(fn `PassiveCatch`
  (locals (BaitItemID :type "Array of Integer") (SpawnWeights :type "Map of Integer to Object Object Reference") (ChanceResult :type Integer) (ItemToSpawn :type Integer))
  (set `local.SpawnWeights` (`self.InsectSpawnWeights`))
  (set `local.ChanceResult` (`KismetMathLibrary.RandomIntegerInRange` 1 100))
  (bind _values (`BlueprintMapLibrary.Map_Values` (`local.SpawnWeights`)))
  (for (_array_element _array_index) _values
    (if (<= (`local.ChanceResult`) _array_element)
      (bind _keys (`BlueprintMapLibrary.Map_Keys` (`local.SpawnWeights`)))
      (set `local.ItemToSpawn` (`KismetArrayLibrary.Array_Get` _keys _array_index))
      (break)))
  (`self.SpawnResultItem` (`local.ItemToSpawn`)))

(fn `SpawnResultItem`
  (params (`Template ID` :type Integer))
  (locals (CurrentInventoryIndex :type Integer :default 0) (`TemplateID to Spawn` :type Integer))
  (bind _returnvalue (`ItemInventory.FindItemByTemplateID` (`self.PlaceableInventory`) (`local.TemplateID to Spawn`) (`local.CurrentInventoryIndex`)))
  (bind _returnvalue_2 (`ItemInventory.GetItem` (`self.PlaceableInventory`) _returnvalue))
  (set `local.TemplateID to Spawn` `Template ID`)
  (if (not (< (`ItemInventory.GetPopulatedItemCount` (`self.PlaceableInventory`) 0 -1) (`ItemInventory.MaxItemCount` (`self.PlaceableInventory`))))
    (set `local.CurrentInventoryIndex` 0)
    (if (!= _returnvalue -1) :!label _label
      (if (< (`GameItem.GetIntStat` _returnvalue_2 "StackSize") (`GameItem.GetIntStat` _returnvalue_2 "MaxStackSize"))
        _
        (else
          (set `local.CurrentInventoryIndex` (+ (`local.CurrentInventoryIndex`) 1))
          (goto _label)))
      (else
        (return))))
  (`ItemInventory.AddItemTemplate` (`self.PlaceableInventory`) (`local.TemplateID to Spawn`) -1 1 false 1.0 -1.0)
  (return))

(fn `UserConstructionScript`
  (`parent.UserConstructionScript`))