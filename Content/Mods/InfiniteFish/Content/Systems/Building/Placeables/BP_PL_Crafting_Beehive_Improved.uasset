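; Improved beehive crafting placeable that periodically produces a fixed item (template 18002) into its own inventory.
; A looping server timer, scaled by TickModifier, drives SpawnResultItem, which adds to a free slot or an unfilled stack; brushes are skipped.
; Inventory add and remove signals restart the timer and show bees with loop audio, while an add that reaches MaxItems stops production and hides and mutes them, all server-side.
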(event `self.ReceiveBeginPlay`
  (`ConanAudioComponent.SetVolumeMultiplier` (`self.CraftingLoopAudio`) 0.0)
  (if (`KismetSystemLibrary.IsServer`)
    (bind _returnvalue (`KismetSystemLibrary.K2_SetTimerDelegate` (delegate `Tick`) (* (`self.Tick Time`) (`self.Tick modifier`)) true))
    (set `self.TimerHandle` _returnvalue)))

(event `Tick`
  (if (not (`self.IsABrush`))
    (`self.SpawnResultItem` 18002)))

(event `self.PlaceableInventory.SignalItemAdded`
  (params (index :type Integer) (item :type "GameItem Object Reference") (srcInventory :type "ItemInventory Object Reference") (srcIndex :type Integer))
  (if (`KismetSystemLibrary.IsServer`)
    (if (== (`ItemInventory.GetItemCount` (`self.PlaceableInventory`)) (`self.Max Items`))
      (`KismetSystemLibrary.K2_ClearAndInvalidateTimerHandle` (`self.TimerHandle`))
      (`SceneComponent.SetVisibility` (`self.bees`) false false)
      (`SceneComponent.SetVisibility` (`self.bees2`) false false)
      (`ConanAudioComponent.SetVolumeMultiplier` (`self.CraftingLoopAudio`) 0.0)
      (else
        (bind _returnvalue (`KismetSystemLibrary.K2_SetTimerDelegate` (delegate `Tick`) (* (`self.Tick Time`) (`self.Tick modifier`)) true :!label _label))
        (set `self.TimerHandle` _returnvalue)
        (`SceneComponent.SetVisibility` (`self.bees`) true true)
        (`SceneComponent.SetVisibility` (`self.bees2`) true true)
        (`ConanAudioComponent.SetVolumeMultiplier` (`self.CraftingLoopAudio`) 1.056324)))))

(event `self.PlaceableInventory.SignalItemRemoved`
  (params (index :type Integer) (item :type "GameItem Object Reference") (dstInventory :type "ItemInventory Object Reference") (dstIndex :type Integer))
  (if (`KismetSystemLibrary.IsServer`)
    (goto _label)))

(fn `GetArtisanThrallInventory`
  (returns (ReturnValue :type "ItemInventory Object Reference"))
  (return null))

(fn `SpawnResultItem`
  (params (templateID :type Integer))
  (locals (`TemplateID to Spawn` :type Integer) (CurrentInventoryIndex :type Integer))
  (bind _returnvalue (`ItemInventory.FindItemByTemplateID` (`self.PlaceableInventory`) (`local.TemplateID to Spawn`) (`local.CurrentInventoryIndex`)))
  (bind _returnvalue_2 (`ItemInventory.GetItem` (`self.PlaceableInventory`) _returnvalue))
  (set `local.TemplateID to Spawn` templateID)
  (if (not (< (`ItemInventory.GetPopulatedItemCount` (`self.PlaceableInventory`) 0 -1) (`ItemInventory.MaxItemCount` (`self.PlaceableInventory`))))
    (set `local.CurrentInventoryIndex` 0)
    (if (!= _returnvalue -1) :!label _label
      (if (< (`GameItem.GetIntStat` _returnvalue_2 "StackSize") (`GameItem.GetIntStat` _returnvalue_2 "MaxStackSize"))
        _
        (else
          (set `local.CurrentInventoryIndex` (+ (`local.CurrentInventoryIndex`) 1))
          (goto _label)))
      (else
        (return))))
  (`ItemInventory.AddItemTemplate` (`self.PlaceableInventory`) (`local.TemplateID to Spawn`) -1 1 false 1.0 -1.0)
  (return))

(fn `UserConstructionScript`
  (`parent.UserConstructionScript`))