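; Placeable fish net, a crafting building variant that yields random catch items by ID.
; Each TickCatch event rolls one in ten and passes the chosen ID to SpawnResultItem.
; Three main items share most of the odds, one roll picks from a secondary five-item pool, and the remaining rolls catch nothing.
; The construction script only calls the parent.
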(event `TickCatch`
  (switch `int` (`KismetMathLibrary.RandomInteger` 10)
    (:`0`
      (`self.SpawnResultItem` 18010 :!label _label))
    (:`1`
      (`self.SpawnResultItem` 18011 :!label _label_2))
    (:`2`
      (`self.SpawnResultItem` 18012 :!label _label_3))
    (:`3`
      (switch `int` (`KismetMathLibrary.RandomInteger` 5)
        (:`0`
          (`self.SpawnResultItem` 80991))
        (:`1`
          (`self.SpawnResultItem` 80992))
        (:`2`
          (`self.SpawnResultItem` 80993))
        (:`3`
          (`self.SpawnResultItem` 80994))
        (:`4`
          (`self.SpawnResultItem` 80995))))
    (:`4`
      (goto _label))
    (:`5`
      (goto _label_2))
    (:`6`
      (goto _label_3))))

(fn `UserConstructionScript`
  (`parent.UserConstructionScript`))